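; Crow1 is a huntable crow that always turns to face the player and can be shot down with arrows.
; OnHit runs once, marking it dead, playing an air-hit animation and sound, enabling physics on its Sphere so it falls, calling ImDead, and incrementing the MotionControllerPawn's Meat.
; When the dead crow's Sphere hits anything other than BP_BaseArrow, physics stops and the ground-impact animation and sound play.
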(event `self.ReceiveBeginPlay`)

(event `self.ReceiveTick`
  (params (DeltaSeconds :type "Float (single-precision)"))
  (`self.K2_SetActorRotation` (`KismetMathLibrary.FindLookAtRotation` (`self.K2_GetActorLocation`) (`self.K2_GetActorLocation` (`GameplayStatics.GetPlayerPawn` 0)))))

(event `self.Sphere.OnComponentHit`
  (params (HitComponent :type "PrimitiveComponent Object Reference") (OtherActor :type "Actor Object Reference") (OtherComp :type "PrimitiveComponent Object Reference") (NormalImpulse :type "Vector Structure") (Hit :type "HitResult Structure (by ref)"))
  ;[1 1 1] 바닥과 충돌
  (if (not (== (`GameplayStatics.GetObjectClass` OtherActor) "/Game/Blueprints/Bow/BP_BaseArrow.BP_BaseArrow_C"))
    (`KismetSystemLibrary.PrintString` "On Component Hit")
    (if (`self.isDead`)
      (`PrimitiveComponent.SetSimulatePhysics` (`self.Sphere`) false)
      (`SkeletalMeshComponent.PlayAnimation` (`self.SkeletalMesh`) "/Game/Ravens_Crows/Animations/Common/Rav_C_Death_Air_Hit_Ground.Rav_C_Death_Air_Hit_Ground" false)
      (`GameplayStatics.PlaySound2D` "/Game/Final_Sound/까마귀_바닥.까마귀_바닥" 1.0 1.0 0.0 null null))))

(fn `On Hit`
  ;[1 1 1] 화살 맞았을 때
  (if (not (`self.isDead`))
    (`KismetSystemLibrary.PrintString` "On Hit")
    (`SkeletalMeshComponent.PlayAnimation` (`self.SkeletalMesh`) "/Game/Ravens_Crows/Animations/Common/Rav_C_Death_Air_Hit.Rav_C_Death_Air_Hit" false)
    (`PrimitiveComponent.SetSimulatePhysics` (`self.Sphere`) true)
    (`GameplayStatics.PlaySound2D` "/Game/Final_Sound/까마귀_맞았을때_찐.까마귀_맞았을때_찐" 1.0 1.0 0.0 null null)
    (set `self.isDead` true)
    (`self.ImDead`)
    (bind _asmotion_controller_pawn (cast `/Game/VirtualRealityBP/Blueprints/MotionControllerPawn` (`GameplayStatics.GetPlayerPawn` 0)))
    (`/Engine/EditorBlueprintResources/StandardMacros.IncrementInt` (`/Game/VirtualRealityBP/Blueprints/MotionControllerPawn.meat` _asmotion_controller_pawn))))

(fn `UserConstructionScript`)