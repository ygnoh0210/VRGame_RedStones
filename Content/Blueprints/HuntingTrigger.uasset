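; Hunting area trigger actor that spawns random crows when overlapped, capped at 15 alive.
; An overlap with ActingOn set scatters several crows within each CrowSpawnPoint's sphere bounds, picking classes from CrowType.
; LeftBirds counts spawns and drops through each Crow1's bound ImDead event.
; An overlap at the cap clears ActingOn, so the next one below it only re-arms the trigger.
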(event `self.ReceiveActorBeginOverlap`
  (params (OtherActor :type "Actor Object Reference"))
  (bind _left_birds (`self.Left_birds`))
  (if (< (`self.Left_birds`) 15)
    (if (`self.Acting On`)
      (bind _outactors (`GameplayStatics.GetAllActorsOfClass` "/Game/Blueprints/CrowSpawnPoint.CrowSpawnPoint_C"))
      (bind _output_get (set `self.SpawnPoints` _outactors))
      (for _array_element _output_get
        (for _ (range 5)
          (if (< (`self.Left_birds`) 15)
            (bind _asactor (castclass `Actor` (`|GetArrayItem` (`self.CrowType`) (`KismetMathLibrary.RandomInteger` 3))))
            (bind _returnvalue (`|SpawnActorFromClass` _asactor (`KismetMathLibrary.MakeTransform` (+ (`self.K2_GetActorLocation` _array_element) (* (`KismetMathLibrary.RandomUnitVector`) (`.SphereRadius` (`KismetSystemLibrary.GetComponentBounds` (`/Game/Blueprints/CrowSpawnPoint.Sphere` _array_element)))))) "Undefined" "OverrideRootScale" null null))
            (`/Engine/EditorBlueprintResources/StandardMacros.IncrementInt` _left_birds
              (:`  `
                (bind _ascrow_1 (cast `/Game/Ravens_Crows/Blueprints/Crow1` _returnvalue))
                (`KismetSystemLibrary.PrintString` (`KismetStringLibrary.Conv_IntToString` _left_birds))
                (add `/Game/Ravens_Crows/Blueprints/Crow1.ImDead` _ascrow_1 (delegate `DeadEvent`)))))))
      (set `self.Character` (`GameplayStatics.GetPlayerPawn` 0))
      (else
        (set `self.Acting On` true)))
    (else
      (set `self.Acting On` false))))

(event `DeadEvent`
  (`/Engine/EditorBlueprintResources/StandardMacros.DecrementInt` (`self.Left_birds`)))

(event `self.ReceiveBeginPlay`)

(fn `UserConstructionScript`)